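; Base NPC character Blueprint that walks toward the level's BP_Rock objective and can be temporarily slowed.
; On BeginPlay it finds the rock and runs an AI MoveTo, retrying on request failure and changing NPC state when the move finishes.
; A slow-collision event lowers walk speed, then restores it after a retriggerable delay.
; Tick updates the 2D distance to the objective, printed on screen when debug is enabled.
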(event `self.ReceiveBeginPlay`
  ;[0 0 0 0.5] BeginPlay
  (`self.Set Movement Speed` (`self.Base Walk Speed`))
  (bind _returnvalue (`GameplayStatics.GetActorOfClass` "/Game/Assets/Blueprint/Objective/BP_Rock.BP_Rock_C"))
  (set `self.Objective Actor` _returnvalue)
  (`self.UpdateDistance`)
  (`self.ReUpdateMoveLocation`))

(event `self.ReceiveTick`
  (params (DeltaSeconds :type "Float (single-precision)"))
  ;[0 0 0 0.5] Tick
  (`|ExecutionSequence`
    (:`then_0`
      (`self.UpdateDistance`))
    (:`then_1`
      (`self.DebugSystem`))))

(event `/Game/Assets/Blueprint/Characters/NPCs/Interface/BPI_NPCInterface.OnSlowCollision`
  ;[0 0 0 0.5] Events
  (`KismetSystemLibrary.PrintString` "Slowed")
  (`self.Set Movement Speed` (`self.Slowed Walk Speed`))
  (`KismetSystemLibrary.RetriggerableDelay` (`self.Slowed Timer`))
  (`self.Set Movement Speed` (`self.Base Walk Speed`)))

(event `ReUpdateMoveLocation`
  ;[0 0 0 0.5] Events
  (`AITask_MoveTo.AIMoveTo` (`AIBlueprintHelperLibrary.GetAIController` (`self.GetOwner`)) (0.0 0.0 0.0) (`self.Objective Actor`) 1.0 "Enable"
    (:`OnRequestFailed`
      (`self.ReUpdateMoveLocation`))
    (:`OnMoveFinished`
      (set `self.CurrentNPC State` "NewEnumerator1"))))

(fn `Debug Float`
  (params (Name :type Name) (Value :type "Float (double-precision)") (TextColor :type "LinearColor Structure"))
  (`KismetSystemLibrary.PrintString` (`KismetTextLibrary.Conv_TextToString` (`|FormatText` "{Name} : {Value}" Name Value)) true false TextColor 2.0 Name))

(fn `DebugSystem`
  (if (`self.Show Debug`)
    (`self.Debug Float` "Distance To Obj" (`self.DistanceToObjective`) (struct :`G` 1.0 :`B` 0.275936 :`A` 1.0))))

(fn `Set Movement Speed`
  (params (`Max Walk Speed` :type "Float (single-precision)"))
  (set `CharacterMovementComponent.MaxWalkSpeed` `Max Walk Speed` (`self.CharacterMovement`)))

(fn `UpdateDistance`
  (set `self.DistanceToObjective` (`KismetMathLibrary.Vector_Distance2D` (`self.K2_GetActorLocation`) (`self.K2_GetActorLocation` (`self.Objective Actor`)))))

(fn `UserConstructionScript`
  (`parent.UserConstructionScript`))